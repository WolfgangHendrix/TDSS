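; Player projectile Blueprint for the PlexFire shot, layering sound and explosion effects onto its parent class.
; On BeginPlay it runs the parent logic, plays the fire cue as a 2D sound with its own concurrency settings, and binds to its OnDestroyed event.
; When destroyed, it spawns an enlarged P_Explosion particle emitter at its own location.
; The overlap event is a disabled placeholder, and the construction script only calls the parent.
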(event Custom|OnDestroyed_Event
  (params (DestroyedActor :type Actor%20Object%20Reference))
  (Class|GameplayStatics|GetActorArrayAverageLocation (Utilities|Array|MakeArray DestroyedActor))
  (Effects|SpawnEmitteratLocation "/Game/StarterContent/Particles/P_Explosion.P_Explosion" (Transformation|GetActorLocation) "0, 0, 0" "2.000000,2.000000,2.000000"))

(event EventBeginPlay
  (|CallParentFunction)
  (Audio|PlaySound2D "/Game/Audio/snd/sndCuePlexFire.sndCuePlexFire" 1.0 1.0 0.0 "/Game/Audio/sndConc_playerProjectilePlexFire.sndConc_playerProjectilePlexFire" 0 false)
  (EventDispatchers|BindEventtoOnDestroyed (delegate Custom|OnDestroyed_Event)))

(event Collision|EventActorBeginOverlap
  (params (OtherActor :type Actor%20Object%20Reference))
  (|CallParentFunction OtherActor) ; This node is disabled and will not be called.\nDrag off pins to build functionality.
)

(fn ConstructionScript
  (|CallParentFunction))