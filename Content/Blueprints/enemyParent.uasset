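; Base enemy Character that moves steadily along a backward world direction, can fire projectiles and explodes on death.
; Tick feeds reversed movement input, with walk speed set from FwdVelocity on BeginPlay.
; If CanShoot is set, firing starts after a short delay as a Gate loop that spawns projectiles at FireRate intervals until EndFiring closes it.
; HealthCheck plays explosion sound and Niagara effect, then destroys the actor at zero health.
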(event Custom|Start%20Firing
  (Utilities|FlowControl|Sequence
    (:then_0
      (goto _label Open))
    (:then_1
      (Utilities|FlowControl|Gate true :!label _label
        (:Exit
          (Utilities|FlowControl|Sequence
            (:then_0
              (Game|SpawnActorfromClass (Variables|Default|GetprojectileActor) (Math|Transform|MakeTransform (Transformation|GetWorldLocation (Variables|Character|GetMesh)) "0.000000,90.000000,0.000000") "Undefined" "MultiplyWithRoot" 0 0))
            (:then_1
              (Utilities|FlowControl|Delay (* (Math|Float|MakeLiteralFloat 1.0) (Variables|Default|GetfireRate)))
              (goto _label))))))))

(event Custom|End%20Firing
  (Utilities|FlowControl|Gate true) ; enters at Close
)

(event EventBeginPlay
  (bind _fwdvelocity (Variables|Default|GetfwdVelocity))
  (bind _charactermovement (Variables|Character|GetCharacterMovement))
  (Variables|/Script/Engine.CharacterMovementComponent|SetMaxWalkSpeed _charactermovement _fwdvelocity)
  (Variables|/Script/Engine.CharacterMovementComponent|SetMaxWalkSpeedCrouched _charactermovement _fwdvelocity)
  (Utilities|FlowControl|Delay 1.0)
  (if (Variables|Default|GetcanShoot)
    (CallFunction|StartFiring)))

(event Collision|EventActorBeginOverlap
  (params (OtherActor :type Actor%20Object%20Reference)))

(event EventTick
  (params (DeltaSeconds :type Float%20%28single-precision%29))
  (Pawn|Input|AddMovementInput (Math|Vector|GetForwardVector (Math|Rotator|MakeRotator 0.0 (.Pitch (Math|Rotator|BreakRotator (Pawn|GetControlRotation :!class /Script/Engine.Pawn))) 0.0)) -1.0 false))

(fn ConstructionScript)

(fn HealthCheck
  (if (<= (Variables|Default|Gethealth) 0.0)
    (Variables|Default|SetisAlive false)
    (Audio|PlaySound2D (Variables|Default|GetsndExplosion) 1.0 1.0 0.0 0 0)
    (Niagara|SpawnSystematLocation "/Game/Particles/fx_explosionSpace.fx_explosionSpace" (Transformation|GetActorLocation) "0, 0, 0" "2.000000,2.000000,2.000000")
    (Actor|DestroyActor)))