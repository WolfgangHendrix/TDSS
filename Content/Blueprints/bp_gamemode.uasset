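; Game mode that spawns timed waves of enemies from the GameplayData table, starting shortly after BeginPlay.
; SpawnLoop reads rows by an incrementing counter, waits each row's sequence duration, then calls itself until a row is missing.
; Each enemy's class comes from its own array index, while location, health, score, movement and shooting settings all use the row's first entry.
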(event Custom|Spawn%20Loop
  (bind _returnvalue (Utilities|GetDataTableRow "/Game/Data/gameplayData.gameplayData" (Utilities|String|StringToName (Utilities|String|ToString(Integer) (Variables|Default|GetspawnLoopCounter))))
    (:then
      (bind _output_get (Variables|Default|SetcurrentRowData _returnvalue))
      (Variables|Default|SetspawnDelay (.SeqDuration (Utilities|Struct|BreakgameplayStruct _output_get)))
      (Variables|Default|Setscene (.Scene (Utilities|Struct|BreakgameplayStruct _output_get)))
      (for _index (range 0 (- (.EnemyCount (Utilities|Struct|BreakgameplayStruct _output_get)) 1))
        (bind _returnvalue_2 (Game|SpawnActorfromClass (Utilities|Array|Get(acopy) (Variables|Default|GetenemyClasses) (Utilities|SafeGetArrayElement (.Actor (Utilities|Struct|BreakgameplayStruct _output_get)) _index)) (Math|Transform|MakeTransform (Utilities|SafeGetArrayElement (.Locations (Utilities|Struct|BreakgameplayStruct _output_get)))) "Undefined" "MultiplyWithRoot" 0 (Utilities|SafeGetArrayElement (.Health (Utilities|Struct|BreakgameplayStruct _output_get))) (Utilities|SafeGetArrayElement (.ScoreGive (Utilities|Struct|BreakgameplayStruct _output_get))) (Utilities|SafeGetArrayElement (.Movements (Utilities|Struct|BreakgameplayStruct _output_get))) (Utilities|SafeGetArrayElement (.MoveSpeedMulti (Utilities|Struct|BreakgameplayStruct _output_get))) (.X (Math|Vector|BreakVector (Utilities|SafeGetArrayElement (.XYMulti (Utilities|Struct|BreakgameplayStruct _output_get))))) (.Y (Math|Vector|BreakVector (Utilities|SafeGetArrayElement (.XYMulti (Utilities|Struct|BreakgameplayStruct _output_get))))) (Utilities|SafeGetArrayElement (.Velocity (Utilities|Struct|BreakgameplayStruct _output_get))) (Utilities|SafeGetArrayElement (.CanSheet (Utilities|Struct|BreakgameplayStruct _output_get))) (Utilities|SafeGetArrayElement (.FireRate (Utilities|Struct|BreakgameplayStruct _output_get))) 0 0))
        (Utilities|Array|AddUnique (Variables|Default|GetenemyJustSpawned) _returnvalue_2))
      (bind _result (Math|Integer|IncrementInt (Variables|Default|GetspawnLoopCounter))
        (:%20%20
          (Variables|Default|SetspawnLoopCounter _result)
          (Utilities|FlowControl|RetriggerableDelay (Variables|Default|GetspawnDelay))
          (Utilities|Array|Clear (Variables|Default|GetenemyJustSpawned))
          (CallFunction|SpawnLoop))))))

(event EventBeginPlay
  (Utilities|FlowControl|Delay 2.0)
  (CallFunction|SpawnLoop))

(event EventTick
  (params (DeltaSeconds :type Float%20%28single-precision%29)))

(fn ConstructionScript)