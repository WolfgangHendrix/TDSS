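; Player ship Blueprint that follows the mouse cursor and fires from two gun sockets.
; Tick deprojects the cursor to world space and interpolates the actor toward it at Z zero, printing the screen position.
; Primary twin shots and a slower six-projectile spread repeat through Gate and Delay loops; older alternating-fire logic is disconnected.
; HealthCheck clears IsAlive, spawns an explosion and hides the mesh.
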(event Custom|CustomEvent
  (bind _mesh (Variables|Character|GetMesh))
  (bind _projectileplexfire (Variables|Default|GetprojectilePlexFire))
  (bind _returnvalue (Transformation|GetSocketLocation _mesh "gunLeft"))
  (bind _returnvalue_2 (Transformation|GetSocketLocation _mesh "gunRight"))
  ;[1 1 1] Secondary Fire
  (if (not (Variables|Default|GetlockFire))
    (if (Variables|Default|GetcanFire)
      (Utilities|FlowControl|Sequence
        (:then_0
          (goto _label Open))
        (:then_1
          (Utilities|FlowControl|Gate false :!label _label
            (:Exit
              (Utilities|FlowControl|Sequence
                (:then_0
                  _)
                (:then_1
                  (Utilities|FlowControl|Delay (Math|Float|Clamp(Float) (* (* (Variables|Default|GetfireRate) (Variables|Default|GetfireRateMulti)) 4.0) 0.033) :!label _label_2)
                  (Variables|Default|SetcanFire true)
                  (goto _label)))))))
      (else
        (Utilities|FlowControl|Sequence
          (:then_0
            (goto _label Open))
          (:then_1
            (goto _label_2)))))
    ;[1 1 1] Plex Fire
    (Game|SpawnActorfromClass _projectileplexfire (Math|Transform|MakeTransform _returnvalue "0.000000,-110.000000,0.000000" "0.800000,0.800000,0.800000") "Undefined" "MultiplyWithRoot" 0 0)
    (Game|SpawnActorfromClass _projectileplexfire (Math|Transform|MakeTransform _returnvalue "0.000000,-118.000000,0.000000" "0.800000,0.800000,0.800000") "Undefined" "MultiplyWithRoot" 0 0)
    (Game|SpawnActorfromClass _projectileplexfire (Math|Transform|MakeTransform _returnvalue "0.000000,-102.000000,0.000000" "0.800000,0.800000,0.800000") "Undefined" "MultiplyWithRoot" 0 0)
    (Game|SpawnActorfromClass _projectileplexfire (Math|Transform|MakeTransform _returnvalue_2 "0.000000,-80.000000,0.000000" "0.800000,0.800000,0.800000") "Undefined" "MultiplyWithRoot" 0 0)
    (Game|SpawnActorfromClass _projectileplexfire (Math|Transform|MakeTransform _returnvalue_2 "0.000000,-88.000000,0.000000" "0.800000,0.800000,0.800000") "Undefined" "MultiplyWithRoot" 0 0)
    (Game|SpawnActorfromClass _projectileplexfire (Math|Transform|MakeTransform _returnvalue_2 "0.000000,-72.000000,0.000000" "0.800000,0.800000,0.800000") "Undefined" "MultiplyWithRoot" 0 0)
    (Variables|Default|SetcanFire true)))

(event Custom|CustomEvent_1
  (params (Lock%20Firing%20Input :type Boolean))
  (bind _mesh (Variables|Character|GetMesh))
  (bind _projectileplexfire (Variables|Default|GetprojectilePlexFire))
  (bind _returnvalue (Transformation|GetSocketLocation _mesh "gunLeft"))
  (bind _returnvalue_2 (Transformation|GetSocketLocation _mesh "gunRight"))
  ;[1 1 1] Secondary Fire
  (if Lock%20Firing%20Input
    (Variables|Default|SetlockFire true)
    (Utilities|FlowControl|Gate false) ; enters at Close
  ))

(event Custom|Force%20Firing%20Now
  (bind _mesh (Variables|Character|GetMesh))
  (if (not (Variables|Default|GetlockFire))
    (if (Variables|Default|GetcanFire)
      (Utilities|FlowControl|Sequence
        (:then_0
          (goto _label Open))
        (:then_1
          (Utilities|FlowControl|Gate true :!label _label
            (:Exit
              ;[1 1 1] Removing Flip-flopping code for primary shooters per comic design
              (Utilities|FlowControl|Sequence
                (:then_0
                  _)
                (:then_1
                  (Utilities|FlowControl|Delay (Math|Float|Clamp(Float) (* (Variables|Default|GetfireRate) (Variables|Default|GetfireRateMulti)) 0.033) :!label _label_2)
                  (Variables|Default|SetcanFire true)
                  (goto _label)))))))
      (else
        (Utilities|FlowControl|Sequence
          (:then_0
            (goto _label Open))
          (:then_1
            (goto _label_2)))))
    (Game|SpawnActorfromClass (Variables|Default|Getprojectile) (Math|Transform|MakeTransform (Transformation|GetSocketLocation _mesh "gunLeft") "0.000000,-90.000000,0.000000") "Undefined" "MultiplyWithRoot" 0 (Variables|Default|GetdamageMulti) 3333.0 true true 0)
    (Game|SpawnActorfromClass (Variables|Default|Getprojectile) (Math|Transform|MakeTransform (Transformation|GetSocketLocation _mesh "gunRight") "0.000000,-90.000000,0.000000") "Undefined" "MultiplyWithRoot" 0 (Variables|Default|GetdamageMulti) 3333.0 true true 0)
    (Variables|Default|SetcanFire true)))

(event Custom|Stop%20Firing%20Now
  (params (Lock%20Firing%20Input :type Boolean))
  (bind _mesh (Variables|Character|GetMesh))
  (if Lock%20Firing%20Input
    (Variables|Default|SetlockFire true)
    (Utilities|FlowControl|Gate true) ; enters at Close
  ))

(event EventTick
  (params (DeltaSeconds :type Float%20%28single-precision%29))
  (bind _returnvalue (Class|InputDeviceLibrary|GetPlayerControllerfromInputDevice))
  (bind _returnvalue_2 (Class|WidgetLayoutLibrary|GetMousePositiononViewport))
  (Development|PrintText (Utilities|Text|ToText(String) _returnvalue_2) true true "(R=0.000000,G=0.660000,B=1.000000,A=1.000000)" 1e+01)
  (Transformation|SetActorLocation (Math|Interpolation|VInterpTo (Transformation|GetActorLocation) (Math|Vector|MakeVector (.X (Math|Vector|BreakVector (.WorldPosition (Class|GameplayStatics|DeprojectScreentoWorld _returnvalue _returnvalue_2)))) (.Y (Math|Vector|BreakVector (.WorldPosition (Class|GameplayStatics|DeprojectScreentoWorld _returnvalue _returnvalue_2)))) 0.0) (Utilities|Time|GetWorldDeltaSeconds) 32.0) false false))

(event Input|ActionEvents|InputActionFire
  (params (Key :type Key%20Structure))
  (bind _mesh (Variables|Character|GetMesh))
  (:Pressed
    (if (Variables|Default|GetisAlive)
      (if (not (Variables|Default|GetlockFire))
        (if (Variables|Default|GetcanFire)
          (Utilities|FlowControl|Sequence
            (:then_0
              (goto _label Open))
            (:then_1
              (Utilities|FlowControl|Gate true :!label _label
                (:Exit
                  ;[1 1 1] Removing Flip-flopping code for primary shooters per comic design
                  (Utilities|FlowControl|Sequence
                    (:then_0
                      _)
                    (:then_1
                      (Utilities|FlowControl|Delay (Math|Float|Clamp(Float) (* (Variables|Default|GetfireRate) (Variables|Default|GetfireRateMulti)) 0.033) :!label _label_2)
                      (Variables|Default|SetcanFire true)
                      (goto _label)))))))
          (else
            (Utilities|FlowControl|Sequence
              (:then_0
                (goto _label Open))
              (:then_1
                (goto _label_2)))))
        (Game|SpawnActorfromClass (Variables|Default|Getprojectile) (Math|Transform|MakeTransform (Transformation|GetSocketLocation _mesh "gunLeft") "0.000000,-90.000000,0.000000") "Undefined" "MultiplyWithRoot" 0 (Variables|Default|GetdamageMulti) 3333.0 true true 0)
        (Game|SpawnActorfromClass (Variables|Default|Getprojectile) (Math|Transform|MakeTransform (Transformation|GetSocketLocation _mesh "gunRight") "0.000000,-90.000000,0.000000") "Undefined" "MultiplyWithRoot" 0 (Variables|Default|GetdamageMulti) 3333.0 true true 0)
        (Variables|Default|SetcanFire true))))
  (:Released
    (if (not (Variables|Default|GetlockFire))
      (goto _label Close))))

(event Input|ActionEvents|InputActionSecondaryFire
  (params (Key :type Key%20Structure))
  (bind _mesh (Variables|Character|GetMesh))
  (bind _projectileplexfire (Variables|Default|GetprojectilePlexFire))
  (bind _returnvalue (Transformation|GetSocketLocation _mesh "gunLeft"))
  (bind _returnvalue_2 (Transformation|GetSocketLocation _mesh "gunRight"))
  ;[1 1 1] Secondary Fire
  (:Pressed
    (if (Variables|Default|GetisAlive)
      (if (not (Variables|Default|GetlockFire))
        (if (Variables|Default|GetcanFire)
          (Utilities|FlowControl|Sequence
            (:then_0
              (goto _label Open))
            (:then_1
              (Utilities|FlowControl|Gate false :!label _label
                (:Exit
                  (Utilities|FlowControl|Sequence
                    (:then_0
                      _)
                    (:then_1
                      (Utilities|FlowControl|Delay (Math|Float|Clamp(Float) (* (* (Variables|Default|GetfireRate) (Variables|Default|GetfireRateMulti)) 4.0) 0.033) :!label _label_2)
                      (Variables|Default|SetcanFire true)
                      (goto _label)))))))
          (else
            (Utilities|FlowControl|Sequence
              (:then_0
                (goto _label Open))
              (:then_1
                (goto _label_2)))))
        ;[1 1 1] Plex Fire
        (Game|SpawnActorfromClass _projectileplexfire (Math|Transform|MakeTransform _returnvalue "0.000000,-110.000000,0.000000" "0.800000,0.800000,0.800000") "Undefined" "MultiplyWithRoot" 0 0)
        (Game|SpawnActorfromClass _projectileplexfire (Math|Transform|MakeTransform _returnvalue "0.000000,-118.000000,0.000000" "0.800000,0.800000,0.800000") "Undefined" "MultiplyWithRoot" 0 0)
        (Game|SpawnActorfromClass _projectileplexfire (Math|Transform|MakeTransform _returnvalue "0.000000,-102.000000,0.000000" "0.800000,0.800000,0.800000") "Undefined" "MultiplyWithRoot" 0 0)
        (Game|SpawnActorfromClass _projectileplexfire (Math|Transform|MakeTransform _returnvalue_2 "0.000000,-80.000000,0.000000" "0.800000,0.800000,0.800000") "Undefined" "MultiplyWithRoot" 0 0)
        (Game|SpawnActorfromClass _projectileplexfire (Math|Transform|MakeTransform _returnvalue_2 "0.000000,-88.000000,0.000000" "0.800000,0.800000,0.800000") "Undefined" "MultiplyWithRoot" 0 0)
        (Game|SpawnActorfromClass _projectileplexfire (Math|Transform|MakeTransform _returnvalue_2 "0.000000,-72.000000,0.000000" "0.800000,0.800000,0.800000") "Undefined" "MultiplyWithRoot" 0 0)
        (Variables|Default|SetcanFire true))))
  (:Released
    (if (not (Variables|Default|GetlockFire))
      (goto _label Close))))

(fn ConstructionScript)

(fn HealthCheck
  ;[1 1 1] DEAD if true / DAMAGED if false
  (if (<= (Variables|Default|GetHealth) 0.0)
    (Variables|Default|SetisAlive false))
  (Niagara|SpawnSystematLocation "/Game/Particles/fx_explosionSpace.fx_explosionSpace" (Transformation|GetActorLocation))
  (Rendering|SetVisibility (Variables|Character|GetMesh) false false)
  (Variables|Default|SetisAlive false)
  (CallFunction|StopFiringNow false))